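; Player controller that assigns each player one of two pawns, a walker (Promeneur) or a dog (Chien).
; On the server, BeginPlay caches the first actor of each pawn class, searching for the dog only while the walker reference is unset.
; Server Tick retries whenever it controls neither pawn, possessing the walker if it lacks a controller, otherwise the dog if that is free.
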(event `self.ReceiveBeginPlay`
  ;[1 1 1] Mise en place des pawns
  (`/Engine/EditorBlueprintResources/ActorMacros.Switch Has Authority`
    (:`Authority`
      (`self.SetPromeneur/Chien`))))

(event `self.ReceiveTick`
  (params (DeltaSeconds :type "Float (single-precision)"))
  (bind _returnvalue (`self.K2_GetPawn`))
  (bind _promeneur (`self.Promeneur`))
  (bind _chien (`self.Chien`))
  ;[1 1 1] Vérification de la validité et des pawns
  (`/Engine/EditorBlueprintResources/ActorMacros.Switch Has Authority`
    (:`Authority`
      (`/Engine/EditorBlueprintResources/StandardMacros.IsValid` (`self.K2_GetPawn`)
        (:`Is Valid`
          (if (not (or (== _returnvalue (`self.Chien`)) (== _returnvalue (`self.Promeneur`))))
            (`self.SetPromeneur/Chien` :!label _label)
            ;[1 1 1] Possession du Promeneur
            (`/Engine/EditorBlueprintResources/StandardMacros.IsValid` _promeneur
              (:`Is Valid`
                (`/Engine/EditorBlueprintResources/StandardMacros.IsValid` (`/Game/Blueprints/Pawns/PionPromeneur.New Controller` _promeneur)
                  (:`Is Valid`
                    ;[1 1 1] Possession du chien
                    (`/Engine/EditorBlueprintResources/StandardMacros.IsValid` _chien
                      (:`Is Valid`
                        (`/Engine/EditorBlueprintResources/StandardMacros.IsValid` (`/Game/Blueprints/Pawns/PionChien.New Controller` _chien)
                          (:`Is Not Valid`
                            (`self.Possess` (`self.Chien`)))))))
                  (:`Is Not Valid`
                    (`self.Possess` (`self.Promeneur`))))))))
        (:`Is Not Valid`
          (goto _label))))))

(fn `SetPromeneur/Chien`
  (`/Engine/EditorBlueprintResources/StandardMacros.IsValid` (`self.Promeneur`)
    (:`Is Not Valid`
      (bind _returnvalue (`GameplayStatics.GetActorOfClass` "/Game/Blueprints/Pawns/PionPromeneur.PionPromeneur_C"))
      (set `self.Promeneur` _returnvalue)
      (`/Engine/EditorBlueprintResources/StandardMacros.IsValid` (`self.Chien`)
        (:`Is Not Valid`
          (bind _returnvalue_2 (`GameplayStatics.GetActorOfClass` "/Game/Blueprints/Pawns/PionChien.PionChien_C"))
          (set `self.Chien` _returnvalue_2))))))

(fn `UserConstructionScript`)