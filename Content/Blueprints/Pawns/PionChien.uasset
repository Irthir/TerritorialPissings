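; Dog character pawn (PionChien) tied by a simulated leash to the walker pawn (PionPromeneur), which it looks up at BeginPlay.
; Each tick, the authority prints the distance and Sprint state for debugging.
; Beyond a distance threshold while not sprinting, it turns on capsule physics and applies an acceleration force toward the walker, otherwise turning physics off.
; Possession events store or clear the controller reference; Sprint is only read here.
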(event `self.ReceiveBeginPlay`
  ;[1 1 1] Récupération de la référence de l'autre pawn
  (bind _returnvalue (`GameplayStatics.GetActorOfClass` "/Game/Blueprints/Pawns/PionPromeneur.PionPromeneur_C"))
  (set `self.Promeneur` _returnvalue))

(event `self.ReceiveTick`
  (params (DeltaSeconds :type "Float (single-precision)"))
  (bind _bsprint (`self.bSprint`))
  (bind _returnvalue (`self.K2_GetActorLocation` (`self.Promeneur`)))
  (bind _returnvalue_2 (`self.K2_GetActorLocation` self))
  (bind _returnvalue_3 (`KismetMathLibrary.Vector_Distance` _returnvalue_2 _returnvalue))
  ;[1 1 1] Affichage débug
  (`/Engine/EditorBlueprintResources/ActorMacros.Switch Has Authority`
    (:`Authority`
      (`/Engine/EditorBlueprintResources/StandardMacros.IsValid` (`self.Promeneur`)
        (:`Is Valid`
          (`KismetSystemLibrary.PrintString` (`KismetStringLibrary.Conv_DoubleToString` _returnvalue_3) true true (struct :`G` 0.66 :`B` 1.0 :`A` 1.0) DeltaSeconds)
          ;[1 1 1] Gestion de la traction de la laisse
          (`KismetSystemLibrary.PrintString` (`KismetStringLibrary.Conv_BoolToString` _bsprint))
          (if (and (> _returnvalue_3 1000.0) (not _bsprint))
            (`PrimitiveComponent.SetSimulatePhysics` (`self.CapsuleComponent`) true)
            (`PrimitiveComponent.AddForce` (`MovementComponent.UpdatedPrimitive` (`self.CharacterMovement`)) (* (`KismetMathLibrary.GetDirectionUnitVector` _returnvalue_2 _returnvalue) 1000.0) "None" true)
            (else
              (`PrimitiveComponent.SetSimulatePhysics` (`self.CapsuleComponent`) false))))))))

(event `self.ReceivePossessed`
  (params (NewController :type "Controller Object Reference"))
  ;[1 1 1] Gestion de la possession
  (set `self.New Controller` NewController))

(event `self.ReceiveUnpossessed`
  (params (OldController :type "Controller Object Reference"))
  ;[1 1 1] Gestion de la possession
  (set `self.New Controller` null))

(fn `UserConstructionScript`)