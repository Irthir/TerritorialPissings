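; PionPromeneur is the walker pawn that links itself to the dog pawn with a leash at game start.
; On BeginPlay it spawns a BP_Laisse and snaps the leash's walker-end component to its Mesh.
; It then finds the PionChien, teleports its capsule to the leash's dog end and attaches it there, keeping world rotation.
; A cable-to-collar attachment is left unwired, and the dog's name is printed for debugging.
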(event `self.ReceiveBeginPlay`
  (bind _returnvalue (`|SpawnActorFromClass` "/Game/Blueprints/Actors/BP_Laisse.BP_Laisse_C" (`self.GetTransform` self) "AlwaysSpawn" "OverrideRootScale" null null))
  (set `self.Laisse` _returnvalue)
  (`SceneComponent.K2_AttachToComponent` (`/Game/Blueprints/Actors/BP_Laisse.smPromeneur` (`self.Laisse`)) (`self.Mesh`) "0" "SnapToTarget" "SnapToTarget" "KeepWorld" true)
  (bind _returnvalue_2 (`GameplayStatics.GetActorOfClass` "/Game/Blueprints/Pawns/PionChien.PionChien_C"))
  (set `self.Chien` _returnvalue_2)
  (`SceneComponent.K2_SetWorldLocation` (`Character.CapsuleComponent` (`self.Chien`)) (`SceneComponent.K2_GetComponentLocation` (`/Game/Blueprints/Actors/BP_Laisse.smChien` (`self.Laisse`))) false true)
  (`SceneComponent.K2_AttachToComponent` (`Character.CapsuleComponent` (`self.Chien`)) (`/Game/Blueprints/Actors/BP_Laisse.smChien` (`self.Laisse`)) "0" "SnapToTarget" "KeepWorld" "KeepWorld" true)
  (`KismetSystemLibrary.PrintString` (`KismetSystemLibrary.GetDisplayName` (`self.Chien`))))

(fn `UserConstructionScript`)